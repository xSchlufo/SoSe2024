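; BP_Player is the player character, handling movement, look and an idle camera wobble.
; On BeginPlay it adds the Enhanced Input mapping context, sets camera pitch limits and starts the wobble.
; Movement follows control yaw, while look applies sensitivity and optional Y inversion.
; The Anim_Idle timeline offsets camera height, scaling its amplitude and play rate with horizontal speed relative to max walk speed.
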(event Custom|HeadWobble
  (bind _charactermovement (Variables|Character|GetCharacterMovement))
  (bind _velocity (Variables|/Script/Engine.MovementComponent|GetVelocity _charactermovement))
  (bind _maxwalkspeed (Variables|/Script/Engine.CharacterMovementComponent|GetMaxWalkSpeed _charactermovement))
  (bind _returnvalue (Math|Vector|VectorLengthXY _velocity))
  ;[1 1 1] Idle
  (bind _alpha (Timeline|Anim_Idle Play)
    (:Update
      (Components|Timeline|SetPlayRate (Variables|Default|GetAnim_Idle) (Variables|Default|GetIdle%20Speed))
      (Transformation|SetRelativeLocation (Variables|Default|GetCamera) (Math|Vector|MakeVector 0.0 0.0 (* _alpha (Variables|Default|GetIdleAmount) (Math|Float|MapRangeClamped _returnvalue 0.0 _maxwalkspeed 0.7 1.0))) false false)
      (Variables|Default|SetIdle%20Speed (Math|Float|MapRangeClamped _returnvalue 0.0 _maxwalkspeed 0.2 1.0)))))

(event EventBeginPlay
  (CallFunction|SetupInputs)
  (CallFunction|SetupCameraBounds)
  (CallFunction|HeadWobble))

(event Collision|EventActorBeginOverlap
  (params (OtherActor :type Actor%20Object%20Reference)))

(event EventTick
  (params (DeltaSeconds :type Float%20%28single-precision%29)))

(event Input|EnhancedActionEvents|EnhancedInputActionIA_Move
  (params (ActionValue :type Vector%202D%20Structure) (ElapsedSeconds :type Float%20%28double-precision%29) (TriggeredSeconds :type Float%20%28double-precision%29) (InputAction :type Input%20Action%20Object%20Reference :default "/Game/Inputs/IA_Move.IA_Move"))
  ;[1 1 1] Move
  ;;[1 1 1] Move Up/Down
  (Pawn|Input|AddMovementInput (Math|Vector|GetForwardVector (Math|Rotator|MakeRotator 0.0 0.0 (.yaw (Pawn|GetControlRotation :!class /Script/Engine.Pawn)))) (.x ActionValue) false)
  ;;[1 1 1] Move Right/Left
  (Pawn|Input|AddMovementInput (Math|Vector|GetRightVector (Math|Rotator|MakeRotator 0.0 0.0 (.yaw (Pawn|GetControlRotation :!class /Script/Engine.Pawn)))) (.y ActionValue) false))

(event Input|EnhancedActionEvents|EnhancedInputActionIA_Look
  (params (ActionValue :type Vector%202D%20Structure) (ElapsedSeconds :type Float%20%28double-precision%29) (TriggeredSeconds :type Float%20%28double-precision%29) (InputAction :type Input%20Action%20Object%20Reference :default "/Game/Inputs/IA_Look.IA_Look"))
  ;[1 1 1] Look
  (Pawn|Input|AddControllerYawInput (* (.x ActionValue) (Variables|Default|GetSensLook)))
  (Pawn|Input|AddControllerPitchInput (* (.y ActionValue) (Variables|Default|GetSensLook) (Math|Integer|SelectInt 1 -1 (Variables|Default|GetLookYInvert)))))

(fn ConstructionScript)

(fn SetupInputs
  (bind _returnvalue (Game|GetPlayerController 0))
  (bind _returnvalue_2 (PlayerController|LocalPlayerSubsystems|GetEnhancedInputLocalPlayerSubsystem _returnvalue))
  (Utilities|IsValid _returnvalue_2
    (:Is%20Valid
      (Input|AddMappingContext _returnvalue_2 "/Game/Inputs/IMC_Player.IMC_Player" 0 "(bIgnoreAllPressedKeysUntilRelease=True,bForceImmediately=False,bNotifyUserSettings=False)"))
    (:Is%20Not%20Valid
      (Development|PrintString "BP_Player | Input System not found" true true "(R=0.562500,G=0.000000,B=0.000000,A=1.000000)" 5.0))))

(fn SetupCameraBounds
  (bind _returnvalue (Game|GetPlayerCameraManager 0))
  (Variables|/Script/Engine.PlayerCameraManager|SetViewPitchMin _returnvalue -9e+01)
  (Variables|/Script/Engine.PlayerCameraManager|SetViewPitchMax _returnvalue 9e+01))